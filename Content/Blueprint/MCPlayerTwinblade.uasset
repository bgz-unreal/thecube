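; Player character Blueprint for a twinblade fighter with a three-stage attack combo and a dodge.
; On BeginPlay it spawns two sword actors and attaches them to the left and right hand IK sockets on the mesh.
; Attack and Dodge inputs halt movement and raise timed state flags, with repeated attacks advancing the combo, then Delays clear the flags and restore walking.
; Camera-yaw-relative movement nodes remain in the graph but never run.
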(event `self.ReceiveBeginPlay`
  ;[1 1 1] Sword Respawn System
  (bind _returnvalue (`|SpawnActorFromClass` "/Game/Blueprint/SwordWeaponBlueprint.SwordWeaponBlueprint_C" (`KismetMathLibrary.MakeTransform` (0.0 0.0 0.0)) "AlwaysSpawn" "OverrideRootScale" null null))
  (`self.K2_AttachToComponent` _returnvalue (`self.Mesh`) "ik_left_swordweapon_socket" "SnapToTarget" "SnapToTarget" "SnapToTarget" true)
  (bind _returnvalue_2 (`|SpawnActorFromClass` "/Game/Blueprint/SwordWeaponBlueprint.SwordWeaponBlueprint_C" (`KismetMathLibrary.MakeTransform` (0.0 0.0 0.0)) "AlwaysSpawn" "OverrideRootScale" null null))
  (`self.K2_AttachToComponent` _returnvalue_2 (`self.Mesh`) "ik_right_swordweapon_socket" "SnapToTarget" "SnapToTarget" "SnapToTarget" true))

(event `InputAction|Attack`
  (params (Key :type "Key Structure"))
  ;[1 1 1] Combo System
  (:`Pressed`
    (`CharacterMovementComponent.DisableMovement` (`self.CharacterMovement`))
    (`MovementComponent.StopMovementImmediately` (`self.CharacterMovement`))
    (if (`self.bIsAttacking01`)
      (if (`self.bIsAttacking02`)
        (if (not (`self.bIsAttacking03`))
          (set `self.bIsAttacking03` true)
          (`KismetSystemLibrary.Delay` 2.0)
          (set `self.bIsAttacking03` false)
          (`CharacterMovementComponent.SetMovementMode` (`self.CharacterMovement`) "MOVE_Walking" 0 :!label _label))
        (else
          (set `self.bIsAttacking02` true)
          (`KismetSystemLibrary.Delay` 2.0)
          (set `self.bIsAttacking02` false)
          (goto _label)))
      (else
        (set `self.bIsAttacking01` true)
        (`KismetSystemLibrary.Delay` 2.3)
        (set `self.bIsAttacking01` false)
        (goto _label)))))

(event `InputAction|Dodge`
  (params (Key :type "Key Structure"))
  (bind _charactermovement (`self.CharacterMovement`))
  ;[1 1 1] Dodging
  (:`Pressed`
    (`CharacterMovementComponent.DisableMovement` _charactermovement)
    (`MovementComponent.StopMovementImmediately` _charactermovement)
    (set `self.bIsDodging` true)
    (`KismetSystemLibrary.Delay` 1.0)
    (set `self.bIsDodging` false)
    (`CharacterMovementComponent.SetMovementMode` (`self.CharacterMovement`) "MOVE_Walking" 0)))

(fn `UserConstructionScript`)